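; Enemy AI character Blueprint that tints its mesh with a color defined by its controller's config.
; On possession by an EnemyAIController, it copies the config's EnemyColor into the RepNotify variable MaterialColor.
; OnRep_MaterialColor then creates a dynamic instance for each mesh material and sets its Tint parameter, so the color replicates across the network.
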(event EventBeginPlay
  (|CallParentFunction) ; This node is disabled and will not be called.\nDrag off pins to build functionality.
)

(event Collision|EventActorBeginOverlap
  (params (OtherActor :type Actor%20Object%20Reference))
  (|CallParentFunction OtherActor) ; This node is disabled and will not be called.\nDrag off pins to build functionality.
)

(event EventTick
  (params (DeltaSeconds :type Float%20%28single-precision%29))
  (|CallParentFunction DeltaSeconds) ; This node is disabled and will not be called.\nDrag off pins to build functionality.
)

(event EventPossessed
  (params (NewController :type Controller%20Object%20Reference))
  (bind _asenemy_aicontroller (Utilities|Casting|CastToEnemyAIController NewController))
  (Variables|Default|SetMaterialColor (Variables|/Script/Dodger.EnemyConfig|GetEnemyColor (Variables|/Script/Dodger.EnemyAIController|GetConfig _asenemy_aicontroller))))

(fn ConstructionScript
  (|CallParentFunction))

(fn OnRepMaterialColor
  (bind _mesh (Variables|Character|GetMesh))
  (for (_ _array_index) (Rendering|Material|GetMaterials _mesh)
    (bind _returnvalue (Rendering|Material|CreateDynamicMaterialInstance _mesh _array_index 0 "None" :!class /Script/Engine.PrimitiveComponent))
    (Rendering|Material|SetVectorParameterValue _returnvalue "Tint" (Variables|Default|GetMaterialColor) :!class /Script/Engine.MaterialInstanceDynamic)))